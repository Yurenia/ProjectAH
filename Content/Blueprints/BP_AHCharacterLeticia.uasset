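; Player character Blueprint for Leticia that creates the player HUD and handles interaction with objects in front of the character.
; A looping timer runs a short forward capsule trace against one object type, caching the hit actor and showing or hiding its HUD prompt.
; The Interact event sends the interact message to the cached actor when interaction is allowed.
; The Pasue event is an empty stub.
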(event `self.ReceiveBeginPlay`
  (`|ExecutionSequence`
    (:`then_0`
      (bind _returnvalue (`|CreateWidget` "/Game/UI/PlayerHUD.PlayerHUD_C" (`GameplayStatics.GetPlayerController` 0)))
      (bind _output_get (set `self.HUD Reference` _returnvalue))
      (`UserWidget.AddToViewport` _output_get 0))
    (:`then_1`
      (bind _returnvalue_2 (`KismetSystemLibrary.K2_SetTimer` null "CheckActorTrace" 0.1 true))
      (set `self.InteractCheckTimerHandle` _returnvalue_2))))

(event `CheckActorTrace`
  (bind _returnvalue (`self.K2_GetActorLocation`))
  (bind _interactnotice (`/Game/UI/PlayerHUD.InteractNotice` (`self.HUD Reference`)))
  (bind _interactnotice_2 (`/Game/UI/PlayerHUD.InteractNotice` (`self.HUD Reference`)))
  (bind (_outhit _returnvalue_2) (`KismetSystemLibrary.CapsuleTraceSingleForObjects` _returnvalue (+ _returnvalue (* (`self.GetActorForwardVector`) 110.0)) 0.0 (`CapsuleComponent.GetScaledCapsuleHalfHeight` (`self.CapsuleComponent`)) (`|MakeArray` (enumliteral `EObjectTypeQuery` "ObjectTypeQuery7"))))
  (if _returnvalue_2
    (bind (_bblockinghit _binitialoverlap _time _distance _location _impactpoint _normal _impactnormal _physmat _hitactor) (`GameplayStatics.BreakHitResult` _outhit))
    (if (!= (`self.InteractActor`) _hitactor)
      (set `self.CanInteract` true)
      (bind _output_get (set `self.InteractActor` _hitactor))
      (bind _asinteractable_actor_base (cast `/Game/Blueprints/InteractableActor/InteractableActorBase` _output_get))
      (`TextBlock.SetText` (`/Game/UI/InteractNotice.Message` _interactnotice_2) (`/Game/Blueprints/InteractableActor/InteractableActorBase.InteractMessage` _asinteractable_actor_base))
      (`Widget.SetVisibility` _interactnotice_2 "Visible"))
    (else
      (set `self.CanInteract` false)
      (set `self.InteractActor` null)
      (`TextBlock.SetText` (`/Game/UI/InteractNotice.Message` _interactnotice) "")
      (`Widget.SetVisibility` _interactnotice "Collapsed"))))

(event `self.Interact`
  (if (`self.CanInteract`)
    (message `/Game/Blueprints/Interface/I_CharacterInputInteract.InteractEvent` (`self.InteractActor`))))

(event `self.Pasue`)

(fn `UserConstructionScript`)
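; In-game global GameMode that restores saved profile data into the AHGameInstance when play begins.
; If the GameInstance flags the level as opened from Load Game, BeginPlay takes its SaveGame object reference as the current profile.
; A valid current profile then has its difficulty, slot name and playtime copied back onto the GameInstance, keeping that data valid for the session.
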(event `self.ReceiveBeginPlay`
  ;[1 0 0] GameInstance의 변수를 통해 레벨이 Load Game을 통해 오픈되었는지, 그리고 유효한 프로필 레퍼런스를 소유하고 있는지 확인힙니다.
  ; 프로필 레퍼런스가 유효하면, GameInstance에 프로필 데이터를 할당하여 GameInstace가 유효한 데이터를 보유할 수 있게 합니다.
  (`|ExecutionSequence`
    (:`then_0`
      (bind _asahgame_instance (cast `/Game/Blueprints/GameMode/AHGameInstance` (`GameplayStatics.GetGameInstance`)))
      (if (`/Game/Blueprints/GameMode/AHGameInstance.IsOpenLevelFromLoadGame` _asahgame_instance)
        (set `self.CurrentProfile` (`/Game/Blueprints/GameMode/AHGameInstance.SaveGameObjectReference` _asahgame_instance))))
    (:`then_1`
      (bind _currentprofile (`self.CurrentProfile`)
        (:`then`
          (set `/Game/Blueprints/GameMode/AHGameInstance.Difficulty` (`/Game/Blueprints/GameMode/AHSaveProfile.Difficulty` _currentprofile) _asahgame_instance)
          (set `/Game/Blueprints/GameMode/AHGameInstance.CurrentProfileSlotName` (`/Game/Blueprints/GameMode/AHSaveProfile.ProfileSlotName` _currentprofile) _asahgame_instance)
          (set `/Game/Blueprints/GameMode/AHGameInstance.Playtime` (`/Game/Blueprints/GameMode/AHSaveProfile.Playtime` _currentprofile) _asahgame_instance))
        (:`else`)))))

(fn `UserConstructionScript`
  (`parent.UserConstructionScript`))
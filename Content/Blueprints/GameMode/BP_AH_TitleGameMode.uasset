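; Title-level Game Mode that resets the Game Instance's stage zone on BeginPlay and creates the save profile for a new game on EndPlay.
; When the profile menu was opened for New Game, it builds an AH_SaveProfile with the chosen difficulty and slot name.
; It copies both values and the save object to the Game Instance, then writes the slot.
; Per its comment, Load Game is handled in the in-game level Game Mode's BeginPlay.
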(event `self.ReceiveBeginPlay`
  (`parent.ReceiveBeginPlay`)
  (set `/Game/Blueprints/GameMode/AH_GameInstance.StageZone` "NewEnumerator0" (`self.GameInstanceReference`)))

(event `self.ReceiveEndPlay`
  (params (EndPlayReason :type "EEndPlayReason Enum" :default "Destroyed"))
  (bind _gameinstancereference (`self.GameInstanceReference`))
  (bind _difficulty (`self.Difficulty`))
  (bind _slotname (`self.SlotName`))
  (`parent.ReceiveEndPlay` EndPlayReason)
  ;[1 0 0 1 20] 새 게임을 시작할 때만 실행되어야 합니다. Load Game은 인게임 레벨에 연결된 Game Mode의 Begin Play 이벤트를 통해 실행됩니다.
  (switch `/Game/Blueprints/Enum/E_AH_ProfileMenuOpenType` (`self.ProfileMenuOpenType`)
    (:`NewEnumerator1`
      (`|ExecutionSequence`
        (:`then_0`
          (bind _returnvalue (`GameplayStatics.CreateSaveGameObject` "/Game/Blueprints/GameMode/AH_SaveProfile.AH_SaveProfile_C"))
          (set `/Game/Blueprints/GameMode/AH_SaveProfile.ProfileDifficulty` _difficulty _returnvalue)
          (set `/Game/Blueprints/GameMode/AH_SaveProfile.ProfileSlotName` _slotname _returnvalue))
        (:`then_1`
          (set `/Game/Blueprints/GameMode/AH_GameInstance.InstanceDifficulty` _difficulty _gameinstancereference)
          (set `/Game/Blueprints/GameMode/AH_GameInstance.InstanceSlotName` _slotname _gameinstancereference)
          (bind _output_get (set `/Game/Blueprints/GameMode/AH_GameInstance.SaveGameObjectReference` _returnvalue _gameinstancereference))
          (`GameplayStatics.SaveGameToSlot` _output_get (`/Game/Blueprints/GameMode/AH_GameInstance.InstanceSlotName` _gameinstancereference)))))))

(fn `UserConstructionScript`
  (`parent.UserConstructionScript`))
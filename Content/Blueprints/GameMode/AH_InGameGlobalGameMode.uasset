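; In-game global GameMode that restores the player's profile into the GameInstance when gameplay begins from a title-screen profile selection.
; On BeginPlay, it takes the GameInstance's SaveGame reference as the current profile if the level was opened through Load Game.
; A second Sequence step, gated only on that profile being valid, copies difficulty, slot name and playtime to the GameInstance and clears the load flag.
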(event `self.ReceiveBeginPlay`
  (bind _gameinstancereference (`self.GameInstanceReference`))
  (`parent.ReceiveBeginPlay`)
  ;[1 0 0] 타이틀에서 프로필 선택으로 게임을 시작했을 경우에만 실행되어야 합니다.
  ; GameInstance의 변수를 통해 레벨이 Load Game을 통해 오픈되었는지, 그리고 유효한 프로필 레퍼런스를 소유하고 있는지 확인힙니다.
  ; 프로필 레퍼런스가 유효하면, GameInstance에 프로필 데이터를 할당하여 GameInstace가 유효한 데이터를 보유할 수 있게 합니다.
  (`|ExecutionSequence`
    (:`then_0`
      (if (`/Game/Blueprints/GameMode/AH_GameInstance.IsOpenLevelFromLoadGame` _gameinstancereference)
        (set `self.CurrentProfile` (`/Game/Blueprints/GameMode/AH_GameInstance.SaveGameObjectReference` _gameinstancereference))))
    (:`then_1`
      (bind _currentprofile (`self.CurrentProfile`)
        (:`then`
          (set `/Game/Blueprints/GameMode/AH_GameInstance.Difficulty` (`/Game/Blueprints/GameMode/AH_SaveProfile.ProfileDifficulty` _currentprofile) _gameinstancereference)
          (set `/Game/Blueprints/GameMode/AH_GameInstance.SlotName` (`/Game/Blueprints/GameMode/AH_SaveProfile.ProfileSlotName` _currentprofile) _gameinstancereference)
          (set `/Game/Blueprints/GameMode/AH_GameInstance.Playtime` (`/Game/Blueprints/GameMode/AH_SaveProfile.ProfilePlaytime` _currentprofile) _gameinstancereference)
          (set `/Game/Blueprints/GameMode/AH_GameInstance.IsOpenLevelFromLoadGame` false _gameinstancereference))
        (:`else`)))))

(fn `UserConstructionScript`
  (`parent.UserConstructionScript`))
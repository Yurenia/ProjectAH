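; An interactable test actor that triggers a game save when interacted with.
; Its InteractEvent casts the game instance to AH_GameInstance and passes that instance's SlotName to TestSaveGame, stopping if the cast fails.
; The save logic is not in this graph, and the BeginPlay, overlap and Tick events are disabled placeholders.
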(event `/Game/Blueprints/Interface/I_CharacterInputInteract.InteractEvent`
  (bind _asah_game_instance (cast `/Game/Blueprints/GameMode/AH_GameInstance` (`GameplayStatics.GetGameInstance`)))
  (`/Game/Blueprints/FuntionLibrary/SaveLoadLibrary.TestSaveGame` (`/Game/Blueprints/GameMode/AH_GameInstance.SlotName` _asah_game_instance)))

(fn `UserConstructionScript`
  (`parent.UserConstructionScript`))
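; Test interactable actor that opens a common notice dialog box when its InteractEvent fires.
; It passes a hard-coded test message, a confirm button text key and a widget focus state to CreateCommonNoitceDialogBox.
; It stores the returned dialog and binds the button's click to a custom event, which unbinds the click and removes the dialog from its parent.
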(event `/Game/Blueprints/Interface/I_CharacterInputInteract.InteractEvent`
  (bind (_dialogboxreference _buttonreference) (`/Game/Blueprints/FuntionLibrary/UserInterfaceFunctionLibrary.CreateCommonNoitceDialogBox` (make `/Game/Blueprints/Struct/AH_NoticeDialogBoxElement` "This is dialog box create test \nAlso, this message can use for Multi-line text" "USER_INTERFACE_ConfirmButton")))
  (bind _output_get (set `self.DialogBoxReference` _dialogboxreference))
  (add `Button.OnClicked` _buttonreference (delegate `커스텀이벤트_0`)))

(event `커스텀이벤트_0`
  (clear `Button.OnClicked` (stale `/Game/Blueprints/Interface/I_CharacterInputInteract.InteractEvent` _buttonreference))
  (`Widget.RemoveFromParent` (stale `/Game/Blueprints/Interface/I_CharacterInputInteract.InteractEvent` _output_get)))

(fn `UserConstructionScript`
  (`parent.UserConstructionScript`))
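; Blueprint function library of shared UI helpers that create and show common dialog boxes and the profile, difficulty, pause and options menus.
; Dialog creators also return button references, and the profile menu creator stores its open type on the title game mode.
; Focus helpers switch cursor and input mode, temporarily toggling Leticia's movement as a stopgap.
; Back navigation uses a GameInstance widget stack to collapse and restore widgets, though GetPreviousWidget reads index 0.
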(fn `CallPreviousWidget`
  (params (CurrentWidget :type "UserWidget Object Reference"))
  (`Widget.RemoveFromParent` CurrentWidget)
  (bind _asah_game_instance (cast `/Game/Blueprints/GameMode/AH_GameInstance` (`GameplayStatics.GetGameInstance` null)))
  (bind _widgetstack (`/Game/Blueprints/GameMode/AH_GameInstance.WidgetStack` _asah_game_instance))
  (if (not (`KismetArrayLibrary.Array_IsEmpty` _widgetstack))
    (bind _returnvalue (`KismetArrayLibrary.Array_LastIndex` _widgetstack))
    (`Widget.SetVisibility` (`|GetArrayItem` _widgetstack _returnvalue) "Visible")
    (`KismetArrayLibrary.Array_Remove` _widgetstack _returnvalue)))

(fn `ConfirmButtonEvent`
  (locals (ConfirmSound :type "SoundBase Object Reference" :default "SoundWave'/Game/Music/confirm.confirm'") (TestClickString :type String :default "Button Test"))
  (`GameplayStatics.PlaySound2D` null (`local.ConfirmSound`) 1.0 1.0 0.0 null null))

(fn `CreateCommonNoitceDialogBox`
  (params (NoticeDialogBoxProp :type "/Game/Blueprints/Struct/AH_NoticeDialogBoxElement Structure") (WidgetFocusState :type "/Game/Blueprints/Enum/E_AH_WidgetFocusState Enum" :default "NewEnumerator1"))
  (returns (DialogBoxReference :type "/Game/UI/DialogBox/CommonNoticeDialogBox Object Reference") (ButtonReference :type "Button Object Reference"))
  (bind _returnvalue (`|CreateWidget` "/Game/UI/DialogBox/CommonNoticeDialogBox.CommonNoticeDialogBox_C" (`GameplayStatics.GetPlayerController` null) NoticeDialogBoxProp WidgetFocusState))
  (`|ExecutionSequence`
    (:`then_0`
      (bind _button (`/Game/UI/DialogBox/CommonNoticeDialogBox.GetButtonReference` _returnvalue)))
    (:`then_1`
      (`UserWidget.AddToViewport` _returnvalue 0)
      (return _returnvalue _button))))

(fn `CreateCommonSelectionDialogBox`
  (params (SelectionDialogBoxProp :type "/Game/Blueprints/Struct/AH_SelectionDialogBoxElement Structure") (WidgetFocusState :type "/Game/Blueprints/Enum/E_AH_WidgetFocusState Enum" :default "NewEnumerator1"))
  (returns (DialogBoxReference :type "/Game/UI/DialogBox/CommonSelectionDialogBox Object Reference") (AcceptButtonReference :type "Button Object Reference") (DeclineButtonReference :type "Button Object Reference"))
  (bind _returnvalue (`|CreateWidget` "/Game/UI/DialogBox/CommonSelectionDialogBox.CommonSelectionDialogBox_C" (`GameplayStatics.GetPlayerController` null) SelectionDialogBoxProp WidgetFocusState))
  (`|ExecutionSequence`
    (:`then_0`
      (bind (_acceptbuttonreference _declinebuttonreference) (`/Game/UI/DialogBox/CommonSelectionDialogBox.GetButtonReference` _returnvalue)))
    (:`then_1`
      (`UserWidget.AddToViewport` _returnvalue 0)
      (return _returnvalue _acceptbuttonreference _declinebuttonreference))))

(fn `CreateDifficultyMenu`
  (returns (DifficultyMenuReference :type "/Game/UI/DifficultyMenu/DifficultyMenu Object Reference"))
  (bind _returnvalue (`|CreateWidget` "/Game/UI/DifficultyMenu/DifficultyMenu.DifficultyMenu_C"))
  (`UserWidget.AddToViewport` _returnvalue 0)
  (return _returnvalue))

(fn `CreateOptionsMenu`
  (returns (NewParam :type "/Game/UI/OptionsMenu/OptionsMenu Object Reference"))
  (bind _returnvalue (`|CreateWidget` "/Game/UI/OptionsMenu/OptionsMenu.OptionsMenu_C" (`GameplayStatics.GetPlayerController` null)))
  (`UserWidget.AddToViewport` _returnvalue 0)
  (return _returnvalue))

(fn `CreatePauseMenu`
  (returns (PauseMenuReference :type "/Game/UI/PauseMenu/PauseMenu Object Reference"))
  (bind _returnvalue (`|CreateWidget` "/Game/UI/PauseMenu/PauseMenu.PauseMenu_C" (`GameplayStatics.GetPlayerController` null)))
  (`UserWidget.AddToViewport` _returnvalue 0)
  (return _returnvalue))

(fn `CreateProfileMenu`
  (params (ProfileMenuOpenType :type "/Game/Blueprints/Enum/E_AH_ProfileMenuOpenType Enum" :default "NewEnumerator0"))
  (returns (ProfileMenuInstance :type "/Game/UI/ProfileMenu/ProfileMenu Object Reference"))
  (bind _asbp_ah_title_game_mode (cast `/Game/Blueprints/GameMode/BP_AH_TitleGameMode` (`GameplayStatics.GetGameMode` null)))
  (set `/Game/Blueprints/GameMode/BP_AH_TitleGameMode.ProfileMenuOpenType` ProfileMenuOpenType _asbp_ah_title_game_mode)
  (bind _returnvalue (`|CreateWidget` "/Game/UI/ProfileMenu/ProfileMenu.ProfileMenu_C" (`GameplayStatics.GetPlayerController` null)))
  (`UserWidget.AddToViewport` _returnvalue 0)
  (return _returnvalue))

(fn `GetPreviousWidget`
  (returns (PreviousWidgetReference :type "UserWidget Object Reference"))
  (bind _asah_game_instance (cast `/Game/Blueprints/GameMode/AH_GameInstance` (`GameplayStatics.GetGameInstance` null)))
  (bind _widgetstack (`/Game/Blueprints/GameMode/AH_GameInstance.WidgetStack` _asah_game_instance))
  (if (`KismetArrayLibrary.Array_IsValidIndex` _widgetstack)
    (return (`|GetArrayItem` _widgetstack))))

(fn `InFocusWidget`
  (bind _returnvalue (`GameplayStatics.GetPlayerController` null))
  (set `PlayerController.bShowMouseCursor` true _returnvalue)
  (`WidgetBlueprintLibrary.SetInputMode_UIOnlyEx` _returnvalue null "LockAlways")
  ;[1 1 1] 임시방편
  (bind _asbp_ah_character_leticia (cast `/Game/Blueprints/BP_AH_CharacterLeticia` (`GameplayStatics.GetPlayerCharacter` null)))
  (`CharacterMovementComponent.SetMovementMode` (`Character.CharacterMovement` _asbp_ah_character_leticia) "MOVE_None" 0))

(fn `OutFocusWidget`
  (bind _returnvalue (`GameplayStatics.GetPlayerController` null))
  (set `PlayerController.bShowMouseCursor` false _returnvalue)
  (`WidgetBlueprintLibrary.SetInputMode_GameOnly` _returnvalue)
  ;[1 1 1] 임시방편
  (bind _asbp_ah_character_leticia (cast `/Game/Blueprints/BP_AH_CharacterLeticia` (`GameplayStatics.GetPlayerCharacter` null)))
  (`CharacterMovementComponent.SetMovementMode` (`Character.CharacterMovement` _asbp_ah_character_leticia) "MOVE_Walking" 0))

(fn `SaveCurrentWidget`
  (params (CurrentWidget :type "UserWidget Object Reference"))
  (bind _asah_game_instance (cast `/Game/Blueprints/GameMode/AH_GameInstance` (`GameplayStatics.GetGameInstance` null)))
  (`KismetArrayLibrary.Array_Add` (`/Game/Blueprints/GameMode/AH_GameInstance.WidgetStack` _asah_game_instance) CurrentWidget)
  (`Widget.SetVisibility` CurrentWidget "Collapsed"))
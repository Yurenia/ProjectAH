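; Blueprint function library that saves and loads AH_SaveProfile profiles and handles stage restarts.
; ManualSaveGame adds session times to GameInstance totals, records location and level, then writes the profile's slot; LoadGame hands the profile to AH_GameInstance and opens its saved level.
; RestartStage also updates stage condition and re-entry count before reloading, but crosses the runtime and playtime totals.
; AutoSaveGame is empty; the test save and load use different hardcoded slots.
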(fn `AutoSaveGame`
  (params (ProfileReference :type "/Game/Blueprints/GameMode/AH_SaveProfile Object Reference") (CommonSaveElements :type "/Game/Blueprints/Struct/AH_CommonSaveElements Structure")))

(fn `LoadGame`
  (params (SaveProfileReference :type "/Game/Blueprints/GameMode/AH_SaveProfile Object Reference"))
  ;[1 1 1] 게임을 로딩합니다
  ; 게임 모드의 프로필 레퍼런스를 게임 인스턴스의 프로필 레퍼런스로 반환합니다
  (bind _asah_game_instance (cast `/Game/Blueprints/GameMode/AH_GameInstance` (`GameplayStatics.GetGameInstance` null)))
  (set `/Game/Blueprints/GameMode/AH_GameInstance.SaveGameObjectReference` SaveProfileReference _asah_game_instance)
  (`GameplayStatics.OpenLevel` null (`/Game/Blueprints/GameMode/AH_SaveProfile.LastSaveLevelName` SaveProfileReference)))

(fn `ManualSaveGame`
  (params (ProfileReference :type "/Game/Blueprints/GameMode/AH_SaveProfile Object Reference") (CommonSaveElements :type "/Game/Blueprints/Struct/AH_CommonSaveElements Structure"))
  (locals (ProfileObjectReference :type "/Game/Blueprints/GameMode/AH_SaveProfile Object Reference") (NewLocalVar_0 :type "/Game/Blueprints/Struct/AH_CommonSaveElements Structure") (GameInstanceReference :type "/Game/Blueprints/GameMode/AH_GameInstance Object Reference"))
  (bind (_currentruntime _currentplaytime _currentcharacterlocation _currentlevelname) (break `/Game/Blueprints/Struct/AH_CommonSaveElements` CommonSaveElements))
  (bind _profileobjectreference (`local.ProfileObjectReference`))
  (bind _profileobjectreference_2 (`local.ProfileObjectReference`))
  (set `local.ProfileObjectReference` ProfileReference)
  (bind _asah_game_instance (cast `/Game/Blueprints/GameMode/AH_GameInstance` (`GameplayStatics.GetGameInstance` null)))
  (bind _output_get (set `local.GameInstanceReference` _asah_game_instance))
  (set `/Game/Blueprints/GameMode/AH_SaveProfile.ProfileRuntime` (+ (`/Game/Blueprints/GameMode/AH_GameInstance.InstanceRuntime` _output_get) _currentruntime) _profileobjectreference_2)
  (set `/Game/Blueprints/GameMode/AH_SaveProfile.ProfilePlaytime` (+ (`/Game/Blueprints/GameMode/AH_GameInstance.InstancePlaytime` _output_get) _currentplaytime) _profileobjectreference_2)
  (set `/Game/Blueprints/GameMode/AH_SaveProfile.LastSaveLocation` _currentcharacterlocation _profileobjectreference_2)
  (set `/Game/Blueprints/GameMode/AH_SaveProfile.LastSaveLevelName` _currentlevelname _profileobjectreference_2)
  (bind _output_get_2 (set `/Game/Blueprints/GameMode/AH_GameInstance.SaveGameObjectReference` _profileobjectreference (`local.GameInstanceReference`)))
  (bind _returnvalue (`GameplayStatics.SaveGameToSlot` _output_get_2 (`/Game/Blueprints/GameMode/AH_SaveProfile.ProfileSlotName` _profileobjectreference)))
  (if _returnvalue
    (`KismetSystemLibrary.PrintString` null "Save Success")
    (else
      (`KismetSystemLibrary.PrintString` null "Save Failed"))))

(fn `RestartStage`
  (params (ProfileReference :type "/Game/Blueprints/GameMode/AH_SaveProfile Object Reference") (`Restart Elements` :type "/Game/Blueprints/Struct/AH_RestartStageElements Structure"))
  (locals (ProfileObjectReference :type "/Game/Blueprints/GameMode/AH_SaveProfile Object Reference") (GameInstanceReference :type "/Game/Blueprints/GameMode/AH_GameInstance Object Reference"))
  (bind (_currentruntime _currentplaytime _currentstage _currentlevelname) (break `/Game/Blueprints/Struct/AH_RestartStageElements` `Restart Elements`))
  (bind _profileobjectreference (`local.ProfileObjectReference`))
  (bind _profileobjectreference_2 (`local.ProfileObjectReference`))
  (bind _profileobjectreference_3 (`local.ProfileObjectReference`))
  (bind _profilereentrycount (`/Game/Blueprints/GameMode/AH_SaveProfile.ProfileReEntryCount` _profileobjectreference))
  (set `local.ProfileObjectReference` ProfileReference)
  (bind _asah_game_instance (cast `/Game/Blueprints/GameMode/AH_GameInstance` (`GameplayStatics.GetGameInstance` null)))
  (bind _output_get (set `local.GameInstanceReference` _asah_game_instance))
  (set `/Game/Blueprints/GameMode/AH_SaveProfile.ProfileRuntime` (+ (`/Game/Blueprints/GameMode/AH_GameInstance.InstancePlaytime` _output_get) _currentruntime) _profileobjectreference_3)
  (set `/Game/Blueprints/GameMode/AH_SaveProfile.ProfilePlaytime` (+ (`/Game/Blueprints/GameMode/AH_GameInstance.InstanceRuntime` _output_get) _currentplaytime) _profileobjectreference_3)
  (`BlueprintMapLibrary.Map_Add` (`/Game/Blueprints/GameMode/AH_SaveProfile.ProfileStageCondition` _profileobjectreference) _currentstage "NewEnumerator2")
  (`BlueprintMapLibrary.Map_Add` _profilereentrycount _currentstage (+ (`BlueprintMapLibrary.Map_Find` _profilereentrycount _currentstage) 1))
  (bind _output_get_2 (set `/Game/Blueprints/GameMode/AH_GameInstance.SaveGameObjectReference` _profileobjectreference_2 (`local.GameInstanceReference`)))
  (`GameplayStatics.SaveGameToSlot` _output_get_2 (`/Game/Blueprints/GameMode/AH_SaveProfile.ProfileSlotName` _profileobjectreference_2))
  (`GameplayStatics.OpenLevel` null _currentlevelname))

(fn `TestLoadGame`
  (bind ___worldcontext (`local.__WorldContext`))
  (bind _returnvalue (`GameplayStatics.DoesSaveGameExist` "TestSave"))
  (if _returnvalue
    (bind _returnvalue_2 (`GameplayStatics.LoadGameFromSlot` "TestSave"))
    (bind _asah_save_profile (cast `/Game/Blueprints/GameMode/AH_SaveProfile` _returnvalue_2))
    (`|ExecutionSequence`
      (:`then_0`
        (`KismetSystemLibrary.PrintString` ___worldcontext (`|GetEnumeratorNameAsString` (`/Game/Blueprints/GameMode/AH_SaveProfile.ProfileDifficulty` _asah_save_profile))))
      (:`then_1`
        (`KismetSystemLibrary.PrintString` ___worldcontext (`KismetStringLibrary.Conv_VectorToString` (`/Game/Blueprints/GameMode/AH_SaveProfile.LastSaveLocation` _asah_save_profile))))
      (:`then_2`
        (`KismetSystemLibrary.PrintString` ___worldcontext (`KismetStringLibrary.Conv_NameToString` (`/Game/Blueprints/GameMode/AH_SaveProfile.LastSaveLevelName` _asah_save_profile))))
      (:`then_3`
        (`KismetSystemLibrary.PrintString` ___worldcontext (`KismetStringLibrary.Conv_DoubleToString` (`/Game/Blueprints/GameMode/AH_SaveProfile.ProfileRuntime` _asah_save_profile)))))
    (else
      (`KismetSystemLibrary.PrintString` (`local.__WorldContext`) "Cannot found save file"))))

(fn `TestSaveGame`
  (params (SlotName :type String))
  (locals (SaveInstance :type "/Game/Blueprints/GameMode/AH_SaveProfile Object Reference"))
  (bind _returnvalue (`GameplayStatics.CreateSaveGameObject` "/Game/Blueprints/GameMode/AH_SaveProfile.AH_SaveProfile_C"))
  (bind _output_get (set `local.SaveInstance` _returnvalue))
  (`|ExecutionSequence`
    (:`then_0`
      (bind _returnvalue_2 (`GameplayStatics.GetCurrentLevelName` null))
      (set `/Game/Blueprints/GameMode/AH_SaveProfile.LastSaveLevelName` (`KismetStringLibrary.Conv_StringToName` _returnvalue_2) _output_get))
    (:`then_1`
      (set `/Game/Blueprints/GameMode/AH_SaveProfile.LastSaveLocation` (0.0 0.0 0.0) _output_get))
    (:`then_2`
      (set `/Game/Blueprints/GameMode/AH_SaveProfile.ProfileDifficulty` "NewEnumerator1" _output_get))
    (:`then_3`
      (set `/Game/Blueprints/GameMode/AH_SaveProfile.ProfileRuntime` 0.0 _output_get))
    (:`then_4`
      (bind _returnvalue_3 (`GameplayStatics.SaveGameToSlot` _output_get "ProfileSlot1"))
      (if _returnvalue_3
        (`KismetSystemLibrary.PrintString` null "Save Success")
        (else
          (`KismetSystemLibrary.PrintString` null "Save Fail"))))))